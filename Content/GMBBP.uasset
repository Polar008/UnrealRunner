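; GMBBP is a Blueprint, likely the game mode going by its name, that keeps a points total and shows it on screen.
; BeginPlay creates the PointsInter widget for the first player controller and adds it to the viewport.
; Tick runs through a one-second Delay, so AddScore adds a point about every second.
; AddScore increases Points and passes the new total to the widget's ChangeText.
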(event EventBeginPlay
  (Utilities|IsValid (Variables|Default|GetPointInterface)
    (:Is%20Not%20Valid
      (bind _returnvalue (UserInterface|CreateWidget "/Game/PointsInter.PointsInter_C" (Game|GetPlayerController 0)))
      (bind _output_get (Variables|Default|SetPointInterface _returnvalue))
      (UserInterface|Viewport|AddtoViewport _output_get 0))))

(event EventTick
  (params (DeltaSeconds :type Float%20%28single-precision%29))
  (Utilities|FlowControl|Delay 1.0)
  (CallFunction|AddScore 1))

(fn ConstructionScript)

(fn AddScore
  (params (Score :type Integer))
  (bind _pointinterface (Variables|Default|GetPointInterface))
  (bind _output_get (Variables|Default|SetPoints (+ Score (Variables|Default|GetPoints))))
  (Utilities|IsValid _pointinterface
    (:Is%20Valid
      (Default|ChangeText _pointinterface _output_get))))